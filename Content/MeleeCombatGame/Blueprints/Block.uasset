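; Block ability actor that raises its instigator's shield for as long as the actor exists.
; BeginPlay plays the ability montage at zero rate to hold the pose and shows the "Shield"-tagged box component with collision enabled.
; Destruction stops the montage and hides and disables the shield.
; An AnimTraceListener hit event ends the current ability of the reported ThirdPersonCharacter owner.
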(event OnTraceHitActor(AnimTraceListener)
  (params (ActorOwner :type Actor%20Object%20Reference) (FirstSocketName :type Name :default "None") (SecondSocketName :type Name :default "None") (TraceHit :type Hit%20Result%20Structure) (StrikeDirection :type Vector :default "0, 0, 0") (HitActor :type Actor%20Object%20Reference))
  (bind _asthird_person_character (Utilities|Casting|CastToThirdPersonCharacter ActorOwner))
  (Class|AbilityComponent|EndAbility (Variables|/Game/MeleeCombatGame/Blueprints/ThirdPersonCharacter.ThirdPersonCharacter_C|GetAbility _asthird_person_character)))

(event Collision|EventActorBeginOverlap
  (params (OtherActor :type Actor%20Object%20Reference)))

(event EventBeginPlay
  (bind _ascharacter (Utilities|Casting|CastToCharacter (Game|GetInstigator))
    (:then
      (Animation|PlayAnimMontage _ascharacter (Variables|Default|GetAbilityMontage) 0.0 "Default")
      (Utilities|IsValid (Utilities|Array|Get(acopy) (Actor|GetComponentsbyTag _ascharacter "/Script/Engine.BoxComponent" "Shield"))
        (:Is%20Valid
          (Collision|SetCollisionEnabled (Utilities|Array|Get(acopy) (Actor|GetComponentsbyTag _ascharacter "/Script/Engine.BoxComponent" "Shield")) "QueryAndPhysics")
          (Development|SetHiddeninGame (Utilities|Array|Get(acopy) (Actor|GetComponentsbyTag _ascharacter "/Script/Engine.BoxComponent" "Shield")) false false))))
    (:CastFailed
      (Development|PrintString "No Instigator"))))

(event EventDestroyed
  (bind _ascharacter (Utilities|Casting|CastToCharacter (Game|GetInstigator))
    (:then
      (Animation|StopAnimMontage _ascharacter (Variables|Default|GetAbilityMontage))
      (Utilities|IsValid (Utilities|Array|Get(acopy) (Actor|GetComponentsbyTag _ascharacter "/Script/Engine.BoxComponent" "Shield"))
        (:Is%20Valid
          (Collision|SetCollisionEnabled (Utilities|Array|Get(acopy) (Actor|GetComponentsbyTag _ascharacter "/Script/Engine.BoxComponent" "Shield")) "NoCollision")
          (Development|SetHiddeninGame (Utilities|Array|Get(acopy) (Actor|GetComponentsbyTag _ascharacter "/Script/Engine.BoxComponent" "Shield")) true false))))
    (:CastFailed
      (Development|PrintString "No Instigator"))))

(fn ConstructionScript)