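; Base melee attack actor that plays montages on its instigator Character and destroys itself when they end.
; AnimTraceListener events retime each montage before, during and after the trace, spawn hit effects, notify hit actors and apply point damage from server-received hits.
; Combo requests for the same class are communicated, then wait for trace end and a delay before playing the next stacked montage, refilling from a buffer when empty.
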(event OnTraceEnd(AnimTraceListener)
  (params (MeshComponent :type Skeletal%20Mesh%20Component%20Object%20Reference) (ActorOwner :type Actor%20Object%20Reference) (FirstSocketName :type Name :default "None") (SecondSocketName :type Name :default "None"))
  (bind _montagestackbuffer (Variables|Local|GetMontageStackBuffer))
  ;[1 1 1] Vary the Animation play rate during and after tracing
  (Class|AnimBlueprintFunctionLibrary|PlayMontageTracingSectionwithDuration MeshComponent (Utilities|Array|Get(acopy) _montagestackbuffer (Utilities|Array|LastIndex _montagestackbuffer)) (Variables|PhaseTimings|GetAfterTraceTime) "AfterTrace"))

(event OnServerOwnerHitActor(AnimTraceListener)
  (params (Owner :type Actor%20Object%20Reference) (TraceHit :type Hit%20Result%20Structure) (StrikeDirection :type Vector :default "0, 0, 0") (HitActor :type Actor%20Object%20Reference))
  (bind _self self)
  (bind _basedamage (Variables|Damage|GetBaseDamage))
  ;[1 1 1] Do damage when the server receives a hit from the client
  (bind _aspawn (Utilities|Casting|CastToPawn Owner)
    (:then
      (Game|Damage|ApplyPointDamage HitActor _basedamage StrikeDirection TraceHit (Pawn|GetController _aspawn) _self "/Script/Engine.DamageType"))
    (:CastFailed
      (Game|Damage|ApplyPointDamage HitActor _basedamage StrikeDirection TraceHit 0 _self "/Engine/EngineDamageTypes/DmgTypeBP_Environmental.DmgTypeBP_Environmental_C"))))

(event OnTraceHitActor(AnimTraceListener)
  (params (ActorOwner :type Actor%20Object%20Reference) (FirstSocketName :type Name :default "None") (SecondSocketName :type Name :default "None") (TraceHit :type Hit%20Result%20Structure) (StrikeDirection :type Vector :default "0, 0, 0") (HitActor :type Actor%20Object%20Reference))
  ;[1 1 1] Play effects when hits are detected
  (Class|ITraceHittableActor|OnTraceHitMe(Message) HitActor ActorOwner TraceHit StrikeDirection)
  (CallFunction|PlayEffects TraceHit StrikeDirection))

(event OnTraceStart(AnimTraceListener)
  (params (MeshComponent :type Skeletal%20Mesh%20Component%20Object%20Reference) (ActorOwner :type Actor%20Object%20Reference) (FirstSocketName :type Name :default "None") (SecondSocketName :type Name :default "None"))
  (bind _montagestackbuffer (Variables|Local|GetMontageStackBuffer))
  ;[1 1 1] Vary the Animation play rate during and after tracing
  (Class|AnimBlueprintFunctionLibrary|PlayMontageTracingSectionwithDuration MeshComponent (Utilities|Array|Get(acopy) _montagestackbuffer (Utilities|Array|LastIndex _montagestackbuffer)) (Variables|PhaseTimings|GetDuringTraceTime) "DuringTrace"))

(event Custom|RequestCombo
  (params (AttackToCombo :type Actor%20Class%20Reference))
  ;[1 1 1] Comboing
  (if (and (Combo|CanCombo) (== AttackToCombo (Utilities|GetClass self)))
    (Class|ClientAuthorityAbilityActor|Communicate "Combo")
    (CallFunction|RegisterCombo)))

(event Custom|PlayEffects
  (params (Hit :type Hit%20Result%20Structure) (StrikeVector :type Vector))
  ;[1 1 1] Play effects when hits are detected
  (Effects|SpawnEmitteratLocation "/Game/Vikings/Effects/ParticleSystems/P_Hit.P_Hit" (.ImpactPoint (Collision|BreakHitResult Hit)) (Math|Rotator|MakeRotfromZ (Math|Vector|NegateVector StrikeVector)) "0.500000,0.500000,0.500000" true "AutoRelease"))

(event Custom|RegisterCombo
  ;[1 1 1] Comboing
  (EventDispatchers|AssignOnTraceEnd (Variables|Default|GetAnimTraceListener) (delegate Custom|OnTraceEnd_Event_0)))

(event Custom|OnTraceEnd_Event_0
  (params (MeshComponent :type Skeletal%20Mesh%20Component%20Object%20Reference) (ActorOwner :type Actor%20Object%20Reference) (FirstSocketName :type Name) (SecondSocketName :type Name))
  ;[1 1 1] Comboing
  (EventDispatchers|UnbindEventfromOnTraceEnd (Variables|Default|GetAnimTraceListener) (delegate Custom|OnTraceEnd_Event_0))
  (Utilities|FlowControl|Delay (Variables|Combo|GetComboDelayTime))
  (CallFunction|DoCombo MeshComponent))

(event Custom|OnAllMontageInstancesEnded_Event_0
  ;[1 1 1] Start Ability
  (Actor|DestroyActor))

(event Custom|DoCombo
  (params (Mesh%20Comp :type Skeletal%20Mesh%20Component%20Object%20Reference))
  ;[1 1 1] Comboing
  (bind _next_montage (CallFunction|PopNextMontage))
  (Utilities|IsValid _next_montage
    (:Is%20Valid
      (Class|AnimBlueprintFunctionLibrary|PlayMontageTracingSectionwithDuration Mesh%20Comp _next_montage (Variables|PhaseTimings|GetBeforeTraceTime) "BeforeTrace"))
    (:Is%20Not%20Valid
      (Development|PrintString "No Montage"))))

(event EventBeginPlay
  ;[1 1 1] Start Ability
  (bind _ascharacter (Utilities|Casting|CastToCharacter (Game|GetInstigator))
    (:then
      (bind _next_montage (CallFunction|PopNextMontage))
      (Utilities|IsValid _next_montage
        (:Is%20Valid
          (Class|AnimBlueprintFunctionLibrary|PlayMontageTracingSectionwithDuration (Variables|/Script/Engine.Character|GetMesh _ascharacter) _next_montage (Variables|PhaseTimings|GetBeforeTraceTime) "BeforeTrace")
          (EventDispatchers|AssignOnAllMontageInstancesEnded (Components|SkeletalMesh|GetAnimInstance (Variables|/Script/Engine.Character|GetMesh _ascharacter)) (delegate Custom|OnAllMontageInstancesEnded_Event_0)))
        (:Is%20Not%20Valid
          (Development|PrintString "No Montages")
          (Actor|DestroyActor :!label _label))))
    (:CastFailed
      (Development|PrintString "No Instigator")
      (goto _label))))

(event Collision|EventActorBeginOverlap
  (params (OtherActor :type Actor%20Object%20Reference)))

(event EventTick
  (params (DeltaSeconds :type Float%20%28single-precision%29)))

(event EventOnCommunicate
  (params (NewMessage :type Name :default "None"))
  ;[1 1 1] Comboing
  (switch name NewMessage
    (:Combo
      (CallFunction|RegisterCombo))))

(fn ConstructionScript)

(fn PopNextMontage
  (if (Utilities|Array|IsValidIndex (Variables|Animation|GetMontageStack))
    (bind _output_get (LocalVariables|SetNextMontage (Utilities|Array|Get(acopy) (Variables|Animation|GetMontageStack))))
    (Utilities|Array|Add (Variables|Local|GetMontageStackBuffer) _output_get)
    (Utilities|Array|RemoveIndex (Variables|Animation|GetMontageStack))
    (else
      (Variables|Animation|SetMontageStack (Variables|Local|GetMontageStackBuffer))
      (bind _next_montage (CallFunction|PopNextMontage))
      (LocalVariables|SetNextMontage _next_montage)))
  (return (LocalVariables|GetNextMontage)))

(fn CanCombo
  (return (or (Utilities|Array|IsValidIndex (Variables|Animation|GetMontageStack)) (Variables|Combo|GetCanComboForever))))